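; Magic circle actor, a child of what appears to be the MagicCircleCreatorADV Blueprint, that changes its look when a child movement pawn enters its sphere.
; Tick advances a counter through BTALUpValueInstance and prints it as debug output.
; On overlap, the counter becomes the Scene's uniform scale, and hue, glow, pulse and rotation speed are set to fixed values.
; A delayed load of BP_TestCombat is left unconnected.
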(event `self.ReceiveTick`
  (params (DeltaSeconds :type "Float (single-precision)"))
  (bind _output_get (`/Game/Bear/TurnBase/BattleTurnArenaLibrairy.BTAL-UpValueInstance` (`self.Currant Value`) 50.0 DeltaSeconds))
  (bind _output_get_2 (set `self.Currant Value` _output_get))
  (`KismetSystemLibrary.PrintString` (`KismetStringLibrary.Conv_DoubleToString` _output_get_2)))

(event `self.Sphere.OnComponentBeginOverlap`
  (params (OverlappedComponent :type "PrimitiveComponent Object Reference") (OtherActor :type "Actor Object Reference") (OtherComp :type "PrimitiveComponent Object Reference") (OtherBodyIndex :type Integer) (bFromSweep :type Boolean) (SweepResult :type "HitResult Structure (by ref)"))
  (bind _currant_value (`self.Currant Value`))
  (cast `/Game/Bear/Character/C-ChildMouvementPawn` OtherActor)
  (`SceneComponent.SetRelativeScale3D` (`self.Scene`) (`KismetMathLibrary.MakeVector` _currant_value _currant_value _currant_value))
  (set `self.HUE` 250.0)
  (set `self.Emissive_intensity_%` 45.0)
  (set `self.Pulse_Speed_%` 500.0)
  (set `self.Rotation_Speed_%` 600.0)
  (`KismetSystemLibrary.PrintString` "Hello"))

(fn `UserConstructionScript`
  (`parent.UserConstructionScript`))